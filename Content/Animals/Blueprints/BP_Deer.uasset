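; BP_Deer is an animal character with switchable fur, normal and torn suits, though its attack and howl use Savage Werewolf montages.
; BeginPlay applies each suit's visibility, and the construction script makes the fur shirt, pants and body follow the main mesh's pose.
; Attack and howl events fire end dispatchers on montage completion or interruption, with howl also setting a flag.
; A speed enum sets walk speed; damage only prints a debug string.
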(event `self.ReceiveBeginPlay`
  (bind _fur_suit (`self.Fur_Suit`))
  (bind _normal_suit (`self.Normal_Suit`))
  (bind _torn_suit (`self.Torn_Suit`))
  (`SceneComponent.SetVisibility` _fur_suit (`SceneComponent.bVisible` _fur_suit) true)
  (`SceneComponent.SetVisibility` _normal_suit (`SceneComponent.bVisible` _normal_suit) true)
  (`SceneComponent.SetVisibility` _torn_suit (`SceneComponent.bVisible` _torn_suit) true))

(event `Howl`
  (`|PlayMontage` (`self.Mesh`) "/Game/Animations/Werewolf/Montages/AM_AS_SavageWerewolf_Howl.AM_AS_SavageWerewolf_Howl"
    (:`OnCompleted`
      _)
    (:`OnInterrupted`
      _))
  (`self.OnHowlEnd`)
  (set `self.bHowled` true))

(event `DefualtAttack`
  (`|PlayMontage` (`self.Mesh`) "/Game/Animations/Werewolf/Montages/AM_AS_SavageWerewolf_Attack_Long.AM_AS_SavageWerewolf_Attack_Long"
    (:`OnCompleted`
      _)
    (:`OnInterrupted`
      _))
  (`self.OnAttackEnd`))

(event `self.ReceiveAnyDamage`
  (params (Damage :type "Float (single-precision)") (DamageType :type "DamageType Object Reference") (InstigatedBy :type "Controller Object Reference") (DamageCauser :type "Actor Object Reference"))
  (`KismetSystemLibrary.PrintString` "Hello"))

(event `SetMovementSpeed`
  (params (Speed :type "/Game/SavageWerewolf/Blueprints/AI/Enums/E_WerewolfSpeed Enum" :default "NewEnumerator0"))
  (set `CharacterMovementComponent.MaxWalkSpeed` (select `/Game/SavageWerewolf/Blueprints/AI/Enums/E_WerewolfSpeed` Speed :`NewEnumerator1` 150.0 :`NewEnumerator2` 300.0 :`NewEnumerator3` 600.0 :!type "Float (single-precision)") (`self.CharacterMovement`)))

(fn `UserConstructionScript`
  (`SkinnedMeshComponent.SetLeaderPoseComponent` (`self.SK_Shirt_Fur`) (`self.Mesh`) false false)
  (`SkinnedMeshComponent.SetLeaderPoseComponent` (`self.SK_Pant_Fur`) (`self.Mesh`) false false)
  (`SkinnedMeshComponent.SetLeaderPoseComponent` (`self.SK_Body_Fur`) (`self.Mesh`) false false))