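; Arrow projectile that damages enemies or stops where it hits and is flagged as retrievable.
; The construction script sets projectile movement speeds from ArrowSpeed.
; On box overlap, Enemy-tagged actors take ArrowDamage and an AI damage report at the player's location, then the arrow is destroyed.
; Other hits, except Barrier-tagged actors, halt the arrow, remove gravity, set CanBeTaken and make noise at the impact point.
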(event `self.ReceiveBeginPlay`
  (bind _asbp_third_person_character (cast `/Game/ThirdPerson/Blueprints/BP_ThirdPersonCharacter` (`GameplayStatics.GetPlayerCharacter` 0)))
  (set `self.Character` _asbp_third_person_character))

(event `self.Box.OnComponentBeginOverlap`
  (params (OverlappedComponent :type "PrimitiveComponent Object Reference") (OtherActor :type "Actor Object Reference") (OtherComp :type "PrimitiveComponent Object Reference") (OtherBodyIndex :type Integer) (bFromSweep :type Boolean) (SweepResult :type "HitResult Structure (by ref)"))
  (bind _returnvalue (`GameplayStatics.GetPlayerCharacter` 0))
  (if (and (!= OtherActor self) (!= OtherActor "/Game/ThirdPerson/Blueprints/BP_ThirdPersonCharacter.BP_ThirdPersonCharacter"))
    (if (`self.ActorHasTag` OtherActor "Enemy")
      (`GameplayStatics.ApplyDamage` OtherActor (`self.ArrowDamage`))
      (`AISense_Damage.ReportDamageEvent` OtherActor _returnvalue (`self.ArrowDamage`) (`self.K2_GetActorLocation` _returnvalue))
      (`self.K2_DestroyActor`)
      (elif (not (`self.ActorHasTag` OtherActor "Barrier"))
        (`MovementComponent.StopMovementImmediately` (`self.ProjectileMovement`))
        (set `ProjectileMovementComponent.ProjectileGravityScale` 0.0 (`self.ProjectileMovement`))
        (set `self.bCanBeTaken` true)
        (`self.MakeNoise` 1.0 null (`self.K2_GetActorLocation`))))))

(fn `UserConstructionScript`
  (bind _projectilemovement (`self.ProjectileMovement`))
  (bind _arrowspeed (`self.ArrowSpeed`))
  (set `ProjectileMovementComponent.InitialSpeed` _arrowspeed _projectilemovement)
  (set `ProjectileMovementComponent.MaxSpeed` _arrowspeed _projectilemovement))