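; AI controller for the Savage Werewolf that runs BT_Werewolf and drives it through a state enum and targets in the Blackboard.
; On possess it starts Passive and copies the pawn's attack and defend radii.
; Sight triggers Attacking on non-Enemy actors, hearing triggers Investigating, and player damage triggers Attacking, or Scared if the player is protected.
; Hours 6 and 18 toggle Sunrise and Sunset through paired DoOnce gates; separate events handle sleeping and waking.
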(event `self.ReceivePossess`
  (params (PossessedPawn :type "Pawn Object Reference"))
  (bind _blackboard (`self.Blackboard`))
  (bind _asbp_savage_werewolf (cast `/Game/SavageWerewolf/Blueprints/BP_SavageWerewolf` PossessedPawn))
  (bind (_attack _defense) (`/Game/SavageWerewolf/Blueprints/BP_SavageWerewolf.GetIdealRange` _asbp_savage_werewolf))
  (`self.RunBehaviorTree` "/Game/SavageWerewolf/Blueprints/AI/BT_Werewolf.BT_Werewolf")
  (`self.SetStateAsPassive`)
  (`BlackboardComponent.SetValueAsFloat` _blackboard (`self.AttackRadiusKeyName`) _attack)
  (`BlackboardComponent.SetValueAsFloat` _blackboard (`self.DefendRadiusKeyName`) _defense))

(event `self.AIPerception.OnPerceptionUpdated`
  (params (UpdatedActors :type "Array of Actor Object Reference (by ref)"))
  (for _array_element UpdatedActors
    (`|ExecutionSequence`
      (:`then_0`
        (bind _sensed (`self.CanSenseActor` _array_element "NewEnumerator1"))
        (if _sensed
          (`self.HandleSensedSight` _array_element)))
      (:`then_1`
        (bind (_sensed_2 _stimulus) (`self.CanSenseActor` _array_element "NewEnumerator2"))
        (if _sensed_2
          (`self.HandleSensedSound` (`.StimulusLocation` (break `AIStimulus` _stimulus)))))
      (:`then_2`
        (bind _sensed_3 (`self.CanSenseActor` _array_element "NewEnumerator3"))
        (if _sensed_3
          (`self.Handle Sensed Damaged` _array_element))))))

(event `/Game/RTSGAME/Core/Interfaces/BPI_WerewolfSchedule.PassHourToWolf`
  (params (Hour :type Integer))
  (if (== Hour 6)
    (`/Engine/EditorBlueprintResources/StandardMacros.DoOnce` false :!label _label
      (:`Completed`
        (`self.SetStateAsSunrise` (`GameplayStatics.GetPlayerCharacter` 0))
        (goto _label_2 :!via `Reset`)))
    (elif (== Hour 18)
      (`/Engine/EditorBlueprintResources/StandardMacros.DoOnce` false :!label _label_2
        (:`Completed`
          (`self.SetStateAsSunset`)
          (goto _label :!via `Reset`))))))

(event `FallAsleep`
  (`self.SetStateAsSleeping`))

(event `Awake`
  (`self.SetStateAsPassive`))

(fn `CanSenseActor`
  (params (Actor :type "Actor Object Reference") (Sense :type "/Game/SavageWerewolf/Blueprints/AI/Enums/E_Senses Enum" :default "NewEnumerator0"))
  (returns (Sensed :type Boolean) (Stimulus :type "AIStimulus Structure"))
  (bind _info (`AIPerceptionComponent.GetActorsPerception` (`self.AIPerception`) Actor))
  (for _array_element (`.LastSensedStimuli` (break `ActorPerceptionBlueprintInfo` _info))
    (bind _returnvalue (`AIPerceptionSystem.GetSenseClassForStimulus` _array_element))
    (if (== _returnvalue (select `/Game/SavageWerewolf/Blueprints/AI/Enums/E_Senses` Sense :`NewEnumerator1` "/Script/AIModule.AISense_Sight" :`NewEnumerator2` "/Script/AIModule.AISense_Hearing" :`NewEnumerator3` "/Script/AIModule.AISense_Damage" :!type "Object Class Reference"))
      (return (`.bSuccessfullySensed` (break `AIStimulus` _array_element)) _array_element))))

(fn `GetCurrentState`
  (returns (E_State :type "/Game/SavageWerewolf/Blueprints/AI/Enums/E_States Enum"))
  (return (cast `/Game/SavageWerewolf/Blueprints/AI/Enums/E_States` (`BlackboardComponent.GetValueAsEnum` (`self.Blackboard`) (`self.StateKeyName`)))))

(fn `Handle Sensed Damaged`
  (params (Actor :type "Actor Object Reference"))
  (bind _asbp_third_person_character (cast `/Game/ThirdPerson/Blueprints/BP_ThirdPersonCharacter` Actor))
  (bind _e_state (`self.GetCurrentState`))
  (switch `/Game/SavageWerewolf/Blueprints/AI/Enums/E_States` _e_state
    (:`NewEnumerator0`
      _)
    (:`NewEnumerator1`
      _)
    (:`NewEnumerator3`
      _)
    (:`NewEnumerator5`
      _))
  (if (`/Game/ThirdPerson/Blueprints/BP_ThirdPersonCharacter.bIsProtected` _asbp_third_person_character)
    (`self.SetStateAsScared` Actor)
    (else
      (`self.SetStateAsAttacking` Actor))))

(fn `HandleSensedSight`
  (params (Actor :type "Actor Object Reference"))
  (bind _e_state (`self.GetCurrentState`))
  (switch `/Game/SavageWerewolf/Blueprints/AI/Enums/E_States` _e_state
    (:`NewEnumerator0`
      _)
    (:`NewEnumerator3`
      _))
  (if (not (`self.ActorHasTag` Actor "Enemy"))
    (`self.SetStateAsAttacking` Actor)))

(fn `HandleSensedSound`
  (params (Location :type "Vector Structure"))
  (bind _e_state (`self.GetCurrentState`))
  (switch `/Game/SavageWerewolf/Blueprints/AI/Enums/E_States` _e_state
    (:`NewEnumerator0`
      _)
    (:`NewEnumerator3`
      _))
  (`self.SetStateAsInvestigating` Location))

(fn `SetStateAsAttacking`
  (params (AttackTarget :type "Actor Object Reference"))
  (`BlackboardComponent.SetValueAsEnum` (`self.Blackboard`) (`self.StateKeyName`) (enumliteral `/Game/SavageWerewolf/Blueprints/AI/Enums/E_States` "NewEnumerator1"))
  (`BlackboardComponent.SetValueAsObject` (`self.Blackboard`) (`self.PlayerKeyName`) AttackTarget)
  (set `self.AttackTarget` AttackTarget))

(fn `SetStateAsInvestigating`
  (params (Location :type "Vector Structure"))
  (`BlackboardComponent.SetValueAsEnum` (`self.Blackboard`) (`self.StateKeyName`) (enumliteral `/Game/SavageWerewolf/Blueprints/AI/Enums/E_States` "NewEnumerator3"))
  (`BlackboardComponent.SetValueAsVector` (`self.Blackboard`) (`self.PointOfInterestKeyName`) Location))

(fn `SetStateAsPassive`
  (`BlackboardComponent.SetValueAsEnum` (`self.Blackboard`) (`self.StateKeyName`) (enumliteral `/Game/SavageWerewolf/Blueprints/AI/Enums/E_States` "NewEnumerator0")))

(fn `SetStateAsScared`
  (params (AttackTarget :type "Actor Object Reference"))
  (`BlackboardComponent.SetValueAsEnum` (`self.Blackboard`) (`self.StateKeyName`) (enumliteral `/Game/SavageWerewolf/Blueprints/AI/Enums/E_States` "NewEnumerator5"))
  (`BlackboardComponent.SetValueAsObject` (`self.Blackboard`) (`self.PlayerKeyName`) AttackTarget)
  (set `self.AttackTarget` AttackTarget))

(fn `SetStateAsSleeping`
  (`BlackboardComponent.SetValueAsEnum` (`self.Blackboard`) (`self.StateKeyName`) (enumliteral `/Game/SavageWerewolf/Blueprints/AI/Enums/E_States` "NewEnumerator7")))

(fn `SetStateAsSunrise`
  (params (AttackTarget :type "Actor Object Reference"))
  (`BlackboardComponent.SetValueAsEnum` (`self.Blackboard`) (`self.StateKeyName`) (enumliteral `/Game/SavageWerewolf/Blueprints/AI/Enums/E_States` "NewEnumerator6"))
  (`BlackboardComponent.SetValueAsObject` (`self.Blackboard`) (`self.PlayerKeyName`) AttackTarget)
  (set `self.AttackTarget` AttackTarget))

(fn `SetStateAsSunset`
  (`BlackboardComponent.SetValueAsEnum` (`self.Blackboard`) (`self.StateKeyName`) (enumliteral `/Game/SavageWerewolf/Blueprints/AI/Enums/E_States` "NewEnumerator8")))

(fn `UserConstructionScript`)